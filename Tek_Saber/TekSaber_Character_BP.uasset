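; Tek Saber creature Blueprint that adds a laser eye attack, implemented by spawning cannonball projectiles.
; BPDoAttack forwards the attack index to the Laserattack event, which acts only on index 2.
; It spawns ProjCannonBall at an eye component's transform, with the selector hardcoded to the right eye.
; A hardcoded-true branch loops through a short Delay, so firing repeats with no stop condition once started.
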(event `Laser attack`
  (params (`Attack Index` :type Integer))
  (bind _right_eye (`self.Right Eye`))
  (bind _left_eye (`self.Left Eye`))
  (if (== `Attack Index` 2)
    (if true
      (`|SpawnActorFromClass` "/Game/PrimalEarth/CoreBlueprints/Projectiles/ProjCannonBall.ProjCannonBall_C" (select `bool` false :`false` (`KismetMathLibrary.MakeTransform` (`SceneComponent.K2_GetComponentLocation` _right_eye) (`SceneComponent.K2_GetComponentRotation` _right_eye)) :`true` (`KismetMathLibrary.MakeTransform` (`SceneComponent.K2_GetComponentLocation` _left_eye) (`SceneComponent.K2_GetComponentRotation` _left_eye))) :!label _label)
      (if true
        (`KismetSystemLibrary.Delay` 0.2)
        (goto _label)))))

(event `self.BPDoAttack`
  (params (AttackIndex :type Integer))
  (`self.Laser attack` AttackIndex))

(fn `UserConstructionScript`
  (`parent.UserConstructionScript`))