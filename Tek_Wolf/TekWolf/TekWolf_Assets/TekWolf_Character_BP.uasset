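; Tek Wolf creature character with a rocket attack and selectable fur colors.
; On BeginPlay the server reads TekWolf ini options to scale health, stamina, weight, melee damage and speed, or disable ranged attacks.
; Attack index 2 fires rockets using inventory ammo; R plays a pulse montage with a movement lock.
; Multi-use entries cycle fur and fluff types, whose OnRep functions swap mesh materials; fuel logic is disconnected.
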(event `self.ReceiveBeginPlay`
  ;[1 1 1] GUS Settings
  (`KismetSystemLibrary.Delay` 0.2)
  (`/Engine/EditorBlueprintResources/ActorMacros.Switch Has Authority`
    (:`Authority`
      (bind _asshootergamemode (cast `ShooterGameMode` (`GameplayStatics.GetGameMode`)))
      (bind _returnvalue (`ShooterGameMode.GetBoolOptionIni` _asshootergamemode "TekWolf" "DisableRanged"))
      (if _returnvalue
        (set `self.DisableRanged` true false)
        (else
          (set `self.DisableRanged` false false)))
      (bind _returnvalue_2 (`ShooterGameMode.GetFloatOptionIni` _asshootergamemode "TekWolf" "HealthMod"))
      (if (>= _returnvalue_2 1.0)
        (if (<= _returnvalue_2 1000.0)
          (set `self.HealthMod` _returnvalue_2)
          (else
            (set `self.HealthMod` 1.0 :!label _label)))
        (else
          (goto _label)))
      (bind _returnvalue_3 (`self.GetCharacterStatusComponent`))
      (bind _returnvalue_4 (* (`PrimalCharacterStatusComponent.BPGetMaxStatusValue` _returnvalue_3 "Health") (`self.HealthMod`)))
      (`PrimalCharacterStatusComponent.SetMaxStatusValue` _returnvalue_3 "Health" _returnvalue_4)
      (`PrimalCharacterStatusComponent.ModifyCurrentStatusValue` _returnvalue_3 "Health" _returnvalue_4 false false false false null false)
      (bind _returnvalue_5 (`ShooterGameMode.GetFloatOptionIni` _asshootergamemode "TekWolf" "StamMod"))
      (if (>= _returnvalue_5 1.0)
        (if (<= _returnvalue_5 1000.0)
          (set `self.StamMod` _returnvalue_5)
          (else
            (set `self.StamMod` 1.0 :!label _label_2)))
        (else
          (goto _label_2)))
      (bind _returnvalue_6 (`self.GetCharacterStatusComponent`))
      (`PrimalCharacterStatusComponent.SetMaxStatusValue` _returnvalue_6 "Stamina" (* (`PrimalCharacterStatusComponent.BPGetMaxStatusValue` _returnvalue_6 "Stamina") (`self.StamMod`)))
      (bind _returnvalue_7 (`ShooterGameMode.GetFloatOptionIni` _asshootergamemode "TekWolf" "WeightMod"))
      (if (>= _returnvalue_7 1.0)
        (if (<= _returnvalue_7 1000.0)
          (set `self.WeightMod` _returnvalue_7)
          (else
            (set `self.WeightMod` 1.0 :!label _label_3)))
        (else
          (goto _label_3)))
      (bind _returnvalue_8 (`self.GetCharacterStatusComponent`))
      (`PrimalCharacterStatusComponent.SetMaxStatusValue` _returnvalue_8 "Weight" (* (`PrimalCharacterStatusComponent.BPGetMaxStatusValue` _returnvalue_8 "Weight") (`self.WeightMod`)))
      (bind _returnvalue_9 (`ShooterGameMode.GetFloatOptionIni` _asshootergamemode "TekWolf" "DamageMod"))
      (if (>= _returnvalue_9 1.0)
        (if (<= _returnvalue_9 1000.0)
          (set `self.DamageMod` _returnvalue_9)
          (else
            (set `self.DamageMod` 1.0 :!label _label_4)))
        (else
          (goto _label_4)))
      (bind _returnvalue_10 (`self.GetCharacterStatusComponent`))
      (`PrimalCharacterStatusComponent.SetMaxStatusValue` _returnvalue_10 "MeleeDamageMultiplier" (* (`PrimalCharacterStatusComponent.BPGetMaxStatusValue` _returnvalue_10 "MeleeDamageMultiplier") (`self.DamageMod`)))
      (bind _returnvalue_11 (`ShooterGameMode.GetFloatOptionIni` _asshootergamemode "TekWolf" "SpeedMod"))
      (if (>= _returnvalue_11 1.0)
        (if (<= _returnvalue_11 1000.0)
          (set `self.SpeedMod` _returnvalue_11)
          (else
            (set `self.SpeedMod` 1.0 :!label _label_5)))
        (else
          (goto _label_5)))
      (bind _returnvalue_12 (`self.GetCharacterStatusComponent`))
      (`PrimalCharacterStatusComponent.SetMaxStatusValue` _returnvalue_12 "SpeedMultiplier" (* (`PrimalCharacterStatusComponent.BPGetMaxStatusValue` _returnvalue_12 "SpeedMultiplier") (`self.SpeedMod`))))))

(event `self.ReceiveTick`
  (params (DeltaSeconds :type "Float (single-precision)"))
  ;[1 1 1] Fuel Check Tick
)

(event `self.BPDoAttack`
  (params (AttackIndex :type Integer))
  (`self.Rocket Aattck` AttackIndex))

(event `self.RidingTick`)

(event `Rocket Aattck`
  (params (`Attack Index` :type Integer))
  (bind _laser (`self.Laser`))
  (bind _returnvalue (`SceneComponent.K2_GetComponentRotation` _laser))
  (if (== `Attack Index` 2)
    (if (`self.DisableRanged`)
      (bind _returnvalue_2 (`self.GetOwnerController`))
      (bind _asshooterplayercontroller (cast `ShooterPlayerController` _returnvalue_2))
      (`ShooterPlayerController.ClientServerNotification` _asshooterplayercontroller "This Freature is disabled on the server!" (struct :`R` 1.0 :`G` 0.008526 :`A` 1.0) 1.5 0.0 null null)
      (`self.StopAnimMontage` "/Game/Mods/Tek_Wolf/TekWolf/TekWolf_Assets/Animations/Rocket_attack/TekWolf-Attack-laser_Montage.TekWolf-Attack-laser_Montage" :!label _label_6)
      (else
        (bind _returnvalue_3 (`PrimalInventoryComponent.BPGetItemOfTemplate` (`self.MyInventoryComponent`) "/Game/PrimalEarth/CoreBlueprints/Weapons/PrimalItemAmmo_Rocket.PrimalItemAmmo_Rocket_C" false false false false false false false false false false))
        (`/Engine/EditorBlueprintResources/StandardMacros.IsValid` _returnvalue_3
          (:`Is Valid`
            (`KismetSystemLibrary.Delay` 1.8)
            (bind _returnvalue_4 (`|SpawnActorFromClass` "/Game/Mods/Tek_Wolf/TekWolf/TekWolf_Assets/ProjRocket_Tek.ProjRocket_Tek_C" (`KismetMathLibrary.MakeTransform` (`SceneComponent.K2_GetComponentLocation` _laser) _returnvalue)))
            (`ShooterProjectile.BPInitVelocity` _returnvalue_4 (`KismetMathLibrary.GetForwardVector` _returnvalue))
            (`self.ForceNetUpdate` false)
            (`PrimalItem.IncrementItemQuantity` _returnvalue_3 -1 true false false false false))
          (:`Is Not Valid`
            (bind _returnvalue_5 (`self.GetOwnerController`))
            (bind _asshooterplayercontroller_2 (cast `ShooterPlayerController` _returnvalue_5))
            (`ShooterPlayerController.ClientServerNotification` _asshooterplayercontroller_2 "No Rockets!" (struct :`R` 0.865 :`A` 1.0) 1.5 5.0 null null)
            (goto _label_6)))))))

(event `Key|R`
  (:`Pressed`
    (if true
      (`KismetSystemLibrary.Delay` 0.2)
      (`self.IsAttacking`)
      (`self.PlayAnimMontage` "/Game/Mods/Tek_Wolf/TekWolf/TekWolf_Assets/Animations/Tek_pulse/TekWolf_Pulse_Montage.TekWolf_Pulse_Montage")
      (set `self.bPreventMovement` true)
      (`KismetSystemLibrary.Delay` 1.5)
      (set `self.bPreventMovement` false))))

(fn `BPGetMultiUseEntries`
  (params (ForPC :type "PlayerController Object Reference") (MultiUseEntries :type "Array of Actor.MultiUseEntry Structure (by ref)"))
  (returns (ReturnValue :type "Array of Actor.MultiUseEntry Structure"))
  (bind _return_use_entries (`self.Return Use Entries`))
  (set `self.Return Use Entries` MultiUseEntries)
  (`KismetArrayLibrary.Array_Add` _return_use_entries (make `Actor.MultiUseEntry` null "Fur Type" 9001))
  (`KismetArrayLibrary.Array_Add` _return_use_entries (make `Actor.MultiUseEntry` null "Fluff type" 9002 1))
  (return (`self.Return Use Entries`)))

(fn `BPTryMultiUse`
  (params (ForPC :type "PlayerController Object Reference") (UseIndex :type Integer))
  (returns (ReturnValue :type Boolean))
  (switch `int` UseIndex
    (:`Default`
      _)
    (:`9001`
      (switch `int` (`self.Fur_Type`)
        (:`0`
          (set `self.Fur_Type` 1 false))
        (:`1`
          (set `self.Fur_Type` 2 false))
        (:`2`
          (set `self.Fur_Type` 3 false))
        (:`3`
          (set `self.Fur_Type` 4 false))
        (:`4`
          (set `self.Fur_Type` 0 false))))
    (:`9002`
      (switch `int` (`self.Fluff_Type`)
        (:`0`
          (set `self.Fluff_Type` 1 false))
        (:`1`
          (set `self.Fluff_Type` 2 false))
        (:`2`
          (set `self.Fluff_Type` 3 false))
        (:`3`
          (set `self.Fluff_Type` 4 false))
        (:`4`
          (set `self.Fluff_Type` 0 false)))))
  (return true))

(fn `OnRep_Fluff_Type`
  (bind _mesh (`self.Mesh`))
  (switch `int` (`self.Fluff_Type`)
    (:`0`
      (`PrimitiveComponent.CreateDynamicMaterialInstance` _mesh 1 "/Game/Mods/Tek_Wolf/TekWolf/TekWolf_Assets/TekWolf_MIC/Fluff/MIC_Fluff.MIC_Fluff"))
    (:`1`
      (`PrimitiveComponent.CreateDynamicMaterialInstance` _mesh 1 "/Game/Mods/Tek_Wolf/TekWolf/TekWolf_Assets/TekWolf_MIC/Additional_Mats/MIC_Fluff_Blue.MIC_Fluff_Blue"))
    (:`2`
      (`PrimitiveComponent.CreateDynamicMaterialInstance` _mesh 1 "/Game/Mods/Tek_Wolf/TekWolf/TekWolf_Assets/TekWolf_MIC/Additional_Mats/MIC_Fluff_Purple.MIC_Fluff_Purple"))
    (:`3`
      (`PrimitiveComponent.CreateDynamicMaterialInstance` _mesh 1 "/Game/Mods/Tek_Wolf/TekWolf/TekWolf_Assets/TekWolf_MIC/Additional_Mats/MIC_Fluff_Green.MIC_Fluff_Green"))
    (:`4`
      (`PrimitiveComponent.CreateDynamicMaterialInstance` _mesh 1 "/Game/Mods/Tek_Wolf/TekWolf/TekWolf_Assets/TekWolf_MIC/Additional_Mats/MIC_Fluff_White.MIC_Fluff_White"))))

(fn `OnRep_Fur_Type`
  (bind _mesh (`self.Mesh`))
  (switch `int` (`self.Fur_Type`)
    (:`0`
      (`PrimitiveComponent.CreateDynamicMaterialInstance` _mesh 0 "/Game/Mods/Tek_Wolf/TekWolf/TekWolf_Assets/TekWolf_MIC/MIC_TekWolfFur.MIC_TekWolfFur"))
    (:`1`
      (`PrimitiveComponent.CreateDynamicMaterialInstance` _mesh 0 "/Game/Mods/Tek_Wolf/TekWolf/TekWolf_Assets/TekWolf_MIC/Additional_Mats/MIC_TekWolfFur_Red.MIC_TekWolfFur_Red"))
    (:`2`
      (`PrimitiveComponent.CreateDynamicMaterialInstance` _mesh 0 "/Game/Mods/Tek_Wolf/TekWolf/TekWolf_Assets/TekWolf_MIC/Additional_Mats/MIC_TekWolfFur_Purple.MIC_TekWolfFur_Purple"))
    (:`3`
      (`PrimitiveComponent.CreateDynamicMaterialInstance` _mesh 0 "/Game/Mods/Tek_Wolf/TekWolf/TekWolf_Assets/TekWolf_MIC/Additional_Mats/MIC_TekWolfFur_Green.MIC_TekWolfFur_Green"))
    (:`4`
      (`PrimitiveComponent.CreateDynamicMaterialInstance` _mesh 0 "/Game/Mods/Tek_Wolf/TekWolf/TekWolf_Assets/TekWolf_MIC/Additional_Mats/MIC_TekWolfFur_White.MIC_TekWolfFur_White"))))

(fn `UserConstructionScript`
  (`parent.UserConstructionScript`))