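; AI controller for the Tek Dragon, a dino boss that disables forced fleeing and spline wandering.
; On authority it runs the behaviour tree and seeds attack blackboard keys, and on possession it overrides the pawn's stasis sphere radius.
; When idle without a target, it alternates two wander states through the attack index, forcing the second at low health.
; It keeps the dragon grounded during a post-landing interval or below its minimum flight health.
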(event EventBeginPlay
  (bind _asprimaldinoaicontroller (Utilities|Casting|CastToPrimalDinoAIController self))
  (bind _returnvalue (Class|PrimalDinoAIController|GetAttackInterval _asprimaldinoaicontroller))
  (bind _returnvalue_2 (Class|PrimalDinoAIController|GetAttackRotationRangeDegrees _asprimaldinoaicontroller))
  (if (Ability|HasAuthority _asprimaldinoaicontroller)
    (AI|RunBehaviorTree (Variables|/Script/ShooterGame.PrimalDinoAIController|GetBehaviourTree _asprimaldinoaicontroller))
    (AI|Components|Blackboard|SetValueasFloat (AI|GetBlackboard _asprimaldinoaicontroller) (Utilities|Name|MakeLiteralName "AttackDestinationOffsetKey") (Variables|/Script/ShooterGame.PrimalDinoAIController|GetAttackDestinationOffset _asprimaldinoaicontroller))
    (AI|Components|Blackboard|SetValueasFloat (AI|GetBlackboard _asprimaldinoaicontroller) (Utilities|Name|MakeLiteralName "AttackRotationRangeKey") _returnvalue_2)
    (AI|Components|Blackboard|SetValueasFloat (AI|GetBlackboard _asprimaldinoaicontroller) (Utilities|Name|MakeLiteralName "AttackIntervalKey") _returnvalue)))

(fn ConstructionScript
  (Variables|Default|SetbDisableForceFlee true)
  (Variables|Default|SetbUseSplineWandering false))

(fn OnPossess
  (params (PossessedPawn :type Pawn%20Object%20Reference))
  (bind _returnvalue (Class|PrimalDinoAIController|GetControllerPawn))
  (if (!= _returnvalue 0)
    (if (!= (Variables|/Script/Engine.Actor|GetStasisCheckComponent _returnvalue) 0)
      (bind _asspherecomponent (Utilities|Casting|CastToSphereComponent (Variables|/Script/Engine.Actor|GetStasisCheckComponent _returnvalue)))
      (Components|Sphere|SetSphereRadius _asspherecomponent (Variables|Default|GetStasisOverrideRadius) true))))

(fn CalculateandSetWonderingAIStateEvent
  (params (StateChanged :type Boolean))
  (LocalVariables|SetisLowHealth false)
  (LocalVariables|SetlocalReturn false)
  (Utilities|FlowControl|Sequence
    (:then_0
      (bind _returnvalue (Class|PrimalDinoAIController|GetControllerPawn))
      (if (!= _returnvalue 0)
        (Utilities|FlowControl|Sequence
          (:then_0
            (bind _asdragon_character_bp_boss_c (Utilities|Casting|CastToDragon_Character_BP_Boss _returnvalue))
            (LocalVariables|SetisLowHealth (<= (/ (Variables|/Script/ShooterGame.PrimalCharacter|GetReplicatedCurrentHealth _asdragon_character_bp_boss_c) (Variables|/Script/ShooterGame.PrimalCharacter|GetReplicatedMaxHealth _asdragon_character_bp_boss_c)) (Variables|/Game/PrimalEarth/Dinos/Dragon/Dragon_Character_BP_Boss.Dragon_Character_BP_Boss_C|GetMinimumHealthRequiredForFlight _asdragon_character_bp_boss_c))))
          (:then_1
            (bind _asprimaldinocharacter (Utilities|Casting|CastToPrimalDinoCharacter _returnvalue))
            (bind _returnvalue_2 (Class|PrimalDinoCharacter|GetActiveState _asprimaldinocharacter))
            (if (Math|Boolean|ANDBoolean (== _returnvalue_2 0) (not (Utilities|IsValid (Variables|/Script/ShooterGame.PrimalDinoCharacter|GetTarget _asprimaldinocharacter))) (== (Variables|/Script/ShooterGame.PrimalDinoCharacter|GetCurrentAttackIndex _asprimaldinocharacter) 255))
              (LocalVariables|SetlocalReturn true)
              (if (or (== (Variables|Default|GetmCurrentWanderState) 0) (LocalVariables|GetisLowHealth))
                (Variables|Default|SetmCurrentWanderState 1)
                (else
                  (Variables|Default|SetmCurrentWanderState 0)))
              (Class|PrimalDinoCharacter|SetCurrentAttackIndex _asprimaldinocharacter (Math|Conversions|ToByte(Integer) (Variables|Default|GetmCurrentWanderState)))
              (if (< (Variables|/Script/ShooterGame.PrimalDinoCharacter|GetCurrentAttackIndex _asprimaldinocharacter) (Math|Conversions|ToByte(Integer) (Utilities|Array|Length (Variables|/Script/ShooterGame.PrimalDinoCharacter|GetAttackInfos _asprimaldinocharacter))))
                (Class|PrimalDinoCharacter|SetState _asprimaldinocharacter (.AttackStateType (Utilities|Struct|BreakDinoAttackInfo (Utilities|Array|Get(acopy) (Variables|/Script/ShooterGame.PrimalDinoCharacter|GetAttackInfos _asprimaldinocharacter) (Math|Conversions|ToInteger(Byte) (Variables|/Script/ShooterGame.PrimalDinoCharacter|GetCurrentAttackIndex _asprimaldinocharacter)))))))
              (if (Variables|Default|GetbTargetChanged)
                (Variables|Default|SetbTargetChanged false)))))))
    (:then_1
      (return (LocalVariables|GetlocalReturn)))))

(fn IsUsingSpline
  (if (Variables|Default|GetbUseSplineWandering)
    _
    (else
      (bind _returnvalue (Class|PrimalDinoAIController|GetControllerPawn))
      (bind _asprimaldinocharacter (Utilities|Casting|CastToPrimalDinoCharacter _returnvalue))))
  (return (== (Variables|/Script/ShooterGame.PrimalDinoCharacter|GetCurrentAttackIndex _asprimaldinocharacter) 0)))

(fn ShouldStayonLand
  (LocalVariables|SetlowHealth false)
  (bind _returnvalue (Class|PrimalDinoAIController|GetControllerPawn))
  (bind _asdragon_character_bp_boss_c (Utilities|Casting|CastToDragon_Character_BP_Boss _returnvalue)
    (:then
      (LocalVariables|SetlowHealth (<= (/ (Variables|/Script/ShooterGame.PrimalCharacter|GetReplicatedCurrentHealth _asdragon_character_bp_boss_c) (Class|PrimalCharacter|GetMaxHealth _asdragon_character_bp_boss_c)) (Variables|/Game/PrimalEarth/Dinos/Dragon/Dragon_Character_BP_Boss.Dragon_Character_BP_Boss_C|GetMinimumHealthRequiredForFlight _asdragon_character_bp_boss_c))))
    (:CastFailed
      _))
  (return (or (< (Class|VictoryCore|TimeSince (Class|Actor|GetWorld) (Math|Conversions|ToFloat(Integer) (Variables|Default|GetAttackLandTime))) (Variables|Default|GetAttackLandInterval)) (LocalVariables|GetlowHealth))))

(fn ReceiveTick
  (params (DeltaSeconds :type Float%20%28single-precision%29)))

(fn OnLosingTargetEvent
  (Variables|Default|SetbShouldScream false))